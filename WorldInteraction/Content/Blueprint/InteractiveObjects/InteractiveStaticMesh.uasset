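; InteractiveStaticMesh is an interactive static mesh object that an interactor can pick up and drop.
; It always allows pickup, switching physics simulation off on the mesh when picked up and back on when dropped.
; Hover, use and drag callbacks are empty stubs, and every interaction callback returns false, including pickup and drop.
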(fn `CanPickup`
  (returns (Pickup :type Boolean))
  (return true))

(fn `OnDrag`
  (params (Interactor :type "/Game/Blueprint/Components/WorldInteractor Object Reference"))
  (returns (Return :type Boolean))
  (return false))

(fn `OnDragEnd`
  (params (Interactor :type "/Game/Blueprint/Components/WorldInteractor Object Reference"))
  (returns (Return :type Boolean))
  (return false))

(fn `OnDragStart`
  (params (Interactor :type "/Game/Blueprint/Components/WorldInteractor Object Reference"))
  (returns (Return :type Boolean))
  (return false))

(fn `OnDrop`
  (params (Interactor :type "/Game/Blueprint/Components/WorldInteractor Object Reference"))
  (returns (Return :type Boolean))
  (`PrimitiveComponent.SetSimulatePhysics` (`self.StaticMeshComponent`) true)
  (return false))

(fn `OnHover`
  (params (Interactor :type "/Game/Blueprint/Components/WorldInteractor Object Reference"))
  (returns (Return :type Boolean))
  (return false))

(fn `OnPickup`
  (params (Interactor :type "/Game/Blueprint/Components/WorldInteractor Object Reference"))
  (returns (Return :type Boolean))
  (`PrimitiveComponent.SetSimulatePhysics` (`self.StaticMeshComponent`) false)
  (return false))

(fn `OnUnHover`
  (params (Interactor :type "/Game/Blueprint/Components/WorldInteractor Object Reference"))
  (returns (Return :type Boolean))
  (return false))

(fn `OnUse`
  (params (Interactor :type "/Game/Blueprint/Components/WorldInteractor Object Reference"))
  (returns (Return :type Boolean))
  (return false))

(fn `UserConstructionScript`)