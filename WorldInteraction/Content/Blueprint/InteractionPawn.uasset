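; InteractionPawn is a VR pawn that lets the player interact with the world through left and right motion controllers.
; Each hand drives its own WorldInteractor: pressing grip picks up and releasing it drops.
; Pressing a trigger uses the hovered object and starts a drag, which stops on release.
; The pawn only routes input, delegating the interaction logic to the interactors.
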(event `Key|MotionController_Left_Grip1`
  (params (Key :type "Key Structure"))
  (bind _worldinteractor_l (`self.WorldInteractor_L`))
  (:`Pressed`
    (`/Game/Blueprint/Components/WorldInteractor.Pickup` _worldinteractor_l))
  (:`Released`
    (`/Game/Blueprint/Components/WorldInteractor.Drop` _worldinteractor_l)))

(event `Key|MotionController_Left_Trigger`
  (params (Key :type "Key Structure"))
  (bind _worldinteractor_l (`self.WorldInteractor_L`))
  (:`Pressed`
    (`/Game/Blueprint/Components/WorldInteractor.UseHoveredObject` _worldinteractor_l)
    (`/Game/Blueprint/Components/WorldInteractor.StartDrag` _worldinteractor_l))
  (:`Released`
    (`/Game/Blueprint/Components/WorldInteractor.StopDrag` _worldinteractor_l)))

(event `Key|MotionController_Right_Grip1`
  (params (Key :type "Key Structure"))
  (bind _worldinteractor_r (`self.WorldInteractor_R`))
  (:`Pressed`
    (`/Game/Blueprint/Components/WorldInteractor.Pickup` _worldinteractor_r))
  (:`Released`
    (`/Game/Blueprint/Components/WorldInteractor.Drop` _worldinteractor_r)))

(event `Key|MotionController_Right_Trigger`
  (params (Key :type "Key Structure"))
  (bind _worldinteractor_r (`self.WorldInteractor_R`))
  (:`Pressed`
    (`/Game/Blueprint/Components/WorldInteractor.UseHoveredObject` _worldinteractor_r)
    (`/Game/Blueprint/Components/WorldInteractor.StartDrag` _worldinteractor_r))
  (:`Released`
    (`/Game/Blueprint/Components/WorldInteractor.StopDrag` _worldinteractor_r)))

(fn `UserConstructionScript`)