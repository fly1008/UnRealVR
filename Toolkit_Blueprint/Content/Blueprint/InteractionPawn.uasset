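; InteractionPawn is a player pawn for interacting with objects through two motion controllers, with keyboard axis input also driving movement.
; Grips pick up and drop through each hand's WorldInteractor, while triggers use the hovered object and start or stop dragging.
; A face button press nudges the player along that controller's forward vector.
; Tick simulates flying with a frame-counted, looping up-and-down movement input.
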(event `InputAxis|MoveRight`
  (params (AxisValue :type "Float (single-precision)"))
  ;[1 1 1] Move with Keyboard
  (`self.MoveRight` AxisValue))

(event `InputAxis|MoveForward`
  (params (AxisValue :type "Float (single-precision)"))
  ;[1 1 1] Move with Keyboard
  (`self.MoveForward` AxisValue))

(event `self.ReceiveTick`
  (params (DeltaSeconds :type "Float (single-precision)"))
  ;[1 1 1] Simulate flying
  (bind _output_get (set `self.Sum` (+ (`self.Sum`) 1)))
  (if (<= _output_get 50)
    (`self.AddMovementInput` (0.0 0.0 0.2) 0.01)
    (elif (<= _output_get 110)
      (`self.AddMovementInput` (0.0 0.0 -0.2) 0.01)
      (else
        (set `self.Sum` 0)))))

(event `Key|MotionController_Right_FaceButton1`
  (params (Key :type "Key Structure"))
  ;[1 1 1] Move Player in direction of MotionControllers
  (:`Pressed`
    (`self.AddMovementInput` (`GameplayStatics.GetPlayerPawn` 0) (`SceneComponent.GetForwardVector` (`self.MotionController_R`)) (`self.Speed`) false)))

(event `Key|MotionController_Left_FaceButton1`
  (params (Key :type "Key Structure"))
  ;[1 1 1] Move Player in direction of MotionControllers
  (:`Pressed`
    (`self.AddMovementInput` (`GameplayStatics.GetPlayerPawn` 0) (`SceneComponent.GetForwardVector` (`self.MotionController_L`)) (`self.Speed`) false)))

(event `Key|MotionController_Left_Grip1`
  (params (Key :type "Key Structure"))
  (bind _worldinteractor_l (`self.WorldInteractor_L`))
  ;[1 1 1] Grap with Left Controller
  (:`Pressed`
    (`/Game/Blueprint/Components/WorldInteractor.Pickup` _worldinteractor_l))
  (:`Released`
    (`/Game/Blueprint/Components/WorldInteractor.Drop` _worldinteractor_l)))

(event `Key|MotionController_Left_Trigger`
  (params (Key :type "Key Structure"))
  (bind _worldinteractor_l (`self.WorldInteractor_L`))
  ;[1 1 1] Use Object with left Controller
  (:`Pressed`
    (`/Game/Blueprint/Components/WorldInteractor.UseHoveredObject` _worldinteractor_l)
    (`/Game/Blueprint/Components/WorldInteractor.StartDrag` _worldinteractor_l))
  (:`Released`
    (`/Game/Blueprint/Components/WorldInteractor.StopDrag` _worldinteractor_l)))

(event `Key|MotionController_Right_Grip1`
  (params (Key :type "Key Structure"))
  (bind _worldinteractor_r (`self.WorldInteractor_R`))
  ;[1 1 1] Grap Object with right Controller
  (:`Pressed`
    (`/Game/Blueprint/Components/WorldInteractor.Pickup` _worldinteractor_r))
  (:`Released`
    (`/Game/Blueprint/Components/WorldInteractor.Drop` _worldinteractor_r)))

(event `Key|MotionController_Right_Trigger`
  (params (Key :type "Key Structure"))
  (bind _worldinteractor_r (`self.WorldInteractor_R`))
  ;[1 1 1] Use Object with right Controller
  (:`Pressed`
    (`/Game/Blueprint/Components/WorldInteractor.UseHoveredObject` _worldinteractor_r)
    (`/Game/Blueprint/Components/WorldInteractor.StartDrag` _worldinteractor_r))
  (:`Released`
    (`/Game/Blueprint/Components/WorldInteractor.StopDrag` _worldinteractor_r)))

(fn `UserConstructionScript`)